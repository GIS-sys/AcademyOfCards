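; BP_WalkingCard is a card actor in WalkingStage that bobs gently up and down.
; Tick accumulates elapsed time and drives the CubeCard component's relative Z with a sine wave, without sweeping.
; The same Tick also creates a new dynamic material instance from MainCardMaterial on slot 0 every frame, setting no parameters on it.
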(event EventBeginPlay)

(event Collision|EventActorBeginOverlap
  (params (OtherActor :type Actor%20Object%20Reference)))

(event EventTick
  (params (DeltaSeconds :type Float%20%28single-precision%29))
  (bind _output_get (Variables|Default|SetTotalTime (+ DeltaSeconds (Variables|Default|GetTotalTime))))
  (Transformation|SetRelativeLocation (Variables|Default|GetCubeCard) (Math|Vector|MakeVector 0.0 0.0 (* (Math|Trig|Sin(Radians) (* _output_get 3.0)) 5.0)) false false)
  (Rendering|Material|CreateDynamicMaterialInstance (Variables|Default|GetCubeCard) 0 (Variables|Default|GetMainCardMaterial) "None" :!class /Script/Engine.PrimitiveComponent))

(fn ConstructionScript)